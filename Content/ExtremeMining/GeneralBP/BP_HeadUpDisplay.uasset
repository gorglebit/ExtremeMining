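; BP_HeadUpDisplay is a HUD that draws a translucent drag-selection box with the mouse, apparently for selecting units.
; Three custom events start the drag, update the current mouse position and end it.
; While drawing, DrawHUD renders the rectangle and queries the actors inside it.
; Its loops compare those actors with SelectedUnits, but the add and remove nodes are disconnected, so the selection never changes here.
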(event Custom|CustomEvent
  (bind _returnvalue (Game|GetPlayerController 0))
  (bind (_locationx _locationy) (Game|Player|GetMousePosition _returnvalue))
  (Variables|Default|SetIsDrawing true)
  (bind _output_get (Variables|Default|SetStartMousePosition (Math|Vector2D|MakeVector2D _locationx _locationy)))
  (Variables|Default|SetCurrentMousePosition _output_get))

(event Custom|CustomEvent_1
  (Variables|Default|SetIsDrawing false))

(event Custom|CustomEvent_2
  (bind _returnvalue (Game|GetPlayerController 0))
  (bind (_locationx _locationy) (Game|Player|GetMousePosition _returnvalue))
  (Variables|Default|SetCurrentMousePosition (Math|Vector2D|MakeVector2D _locationx _locationy)))

(event EventDrawHUD
  (params (SizeX :type Integer) (SizeY :type Integer))
  (bind _startmouseposition (Variables|Default|GetStartMousePosition))
  (bind _currentmouseposition (Variables|Default|GetCurrentMousePosition))
  (if (Variables|Default|GetIsDrawing)
    (HUD|DrawRect "(R=0.000000,G=1.000000,B=1.000000,A=0.300000)" (.x _startmouseposition) (.y _startmouseposition) (- (.x _currentmouseposition) (.x _startmouseposition)) (- (.y _currentmouseposition) (.y _startmouseposition)))
    (bind _output_get (Variables|Default|SetActorsInRectangle (Class|HUD|GetActorsinSelectionRectangle 0 (Variables|Default|GetStartMousePosition) (Variables|Default|GetCurrentMousePosition) false false)))
    (for _array_element _output_get
      _)
    (for _array_element_2 (Variables|Default|GetSelectedUnits)
      (if (== (Utilities|Array|FindItem (Variables|Default|GetActorsInRectangle) _array_element_2) -1)
        _))))

(fn ConstructionScript)