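; Player controller for ExtremeMining that handles mouse input, apparently an unfinished base for building selection and click commands.
; Right-click traces under the cursor, prints the hit actor's name and stores the location unless the actor's class matches an excluded one.
; Left-click only sets a held flag that Tick checks without acting.
; Building selection, interface checks and effect spawning at the clicked location sit in disconnected nodes that never run.
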(event Custom|CustomEvent
  (Utilities|IsValid (Variables|Default|GetSelectedBuilding)))

(event EventTick
  (params (DeltaSeconds :type Float%20%28single-precision%29))
  (Utilities|FlowControl|Sequence
    (:then_0
      (if (Variables|Default|GetIsLeftMousePressed)
        _))))

(event EventBeginPlay)

(event Input|MouseEvents|LeftMouseButton
  (params (Key :type Key%20Structure :default "None"))
  (:Pressed
    (Variables|Default|SetIsLeftMousePressed true))
  (:Released
    (Variables|Default|SetIsLeftMousePressed false)))

(event Input|MouseEvents|RightMouseButton
  (params (Key :type Key%20Structure :default "None"))
  (bind _hitresult (Game|Player|GetHitResultUnderCursorbyChannel "TraceTypeQuery1" true))
  (bind (_bblockinghit _binitialoverlap _time _distance _location _impactpoint _normal _impactnormal _physmat _hitactor) (Collision|BreakHitResult _hitresult))
  (:Pressed
    (Development|PrintString (Utilities|GetDisplayName _hitactor))
    (if (not (== (Utilities|GetClass _hitactor) 0))
      (Variables|Default|SetRightClickLocation _location))))

(fn ConstructionScript)