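; Storage building that displays the Food, Wood and Money stock as rows of cube meshes and labels its name widget "STORAGE".
; BeginPlay sets the building type, gathers ten cubes per resource and builds a shared threshold array in steps of 100.
; Each Set*Storage event shows the cubes whose threshold the resource amount has reached and hides the rest.
; SpawnUpgradeFX spawns an upgrade effect actor above the build mesh.
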(event EventSpawnUpgradeFX
  (Game|SpawnActorfromClass "/Game/ExtremeMining/OtherBP/FX/BP_NSUpgrade.BP_NSUpgrade_C" (Math|Transform|MakeTransform (+ (Transformation|GetWorldLocation (Variables|Default|GetBuildMesh)) "0,0,500.000000") "0, 0, 0" "1.500000,1.500000,1.500000") "Undefined" 0 0))

(event EventSetWoodStorage
  (for (_array_element _array_index) (Variables|Default|GetWoodCubeArray)
    (CallFunction|SetVisibility (Utilities|Array|Get(acopy) (Variables|Default|GetCountArray) _array_index) _array_element (Variables|Default|GetWood))))

(event EventSetMoneyStorage
  (for (_array_element _array_index) (Variables|Default|GetMoneyCubeArray)
    (CallFunction|SetVisibility (Utilities|Array|Get(acopy) (Variables|Default|GetCountArray) _array_index) _array_element (Variables|Default|GetMoney))))

(event EventSetFoodStorage
  (for (_array_element _array_index) (Variables|Default|GetFoodCubeArray)
    (CallFunction|SetVisibility (Utilities|Array|Get(acopy) (Variables|Default|GetCountArray) _array_index) _array_element (Variables|Default|GetFood))))

(event EventBeginPlay
  (Utilities|FlowControl|Sequence
    (:then_0
      (Variables|Default|SetBuildingType 5))
    (:then_1
      (CallFunction|SetFoodCubeArray)
      (CallFunction|SetWoodCubeArray)
      (CallFunction|SetMoneyCubeArray))
    (:then_2
      (CallFunction|SetCountArray))
    (:then_3
      (bind _aswbp_building_name (Utilities|Casting|CastToWBP_BuildingName (UserInterface|GetWidget (Variables|Default|GetBuildingWidget))))
      (Rendering|Components|TextRender|SetText (Variables|/Game/ExtremeMining/UMG/WBP_BuildingName.WBP_BuildingName_C|GetBuildingNameText _aswbp_building_name) "STORAGE"))))

(fn ConstructionScript)

(fn SetVisibility
  (params (Count :type Integer) (Cube :type Scene%20Component%20Object%20Reference) (Resource :type Integer))
  (if (>= Resource Count)
    (Rendering|SetVisibility Cube true false)
    (else
      (Rendering|SetVisibility Cube false false))))

(fn SetFoodCubeArray
  (for _index (range 0 9)
    (Utilities|Array|AddUnique (Variables|Default|GetFoodCubeArray) (Utilities|Select :Index _index :Option%200 (Variables|Default|GetSM_Food_0) :Option%201 (Variables|Default|GetSM_Food_1) :Option%202 (Variables|Default|GetSM_Food_2) :Option%203 (Variables|Default|GetSM_Food_3) :Option%204 (Variables|Default|GetSM_Food_4) :Option%205 (Variables|Default|GetSM_Food_5) :Option%206 (Variables|Default|GetSM_Food_6) :Option%207 (Variables|Default|GetSM_Food_7) :Option%208 (Variables|Default|GetSM_Food_8) :Option%209 (Variables|Default|GetSM_Food_9)))))

(fn SetCountArray
  (for _index (range 0 9)
    (Utilities|Array|AddUnique (Variables|Default|GetCountArray) (LocalVariables|GetCount))
    (LocalVariables|SetCount (+ (LocalVariables|GetCount) 100))))

(fn SetWoodCubeArray
  (for _index (range 0 9)
    (Utilities|Array|AddUnique (Variables|Default|GetWoodCubeArray) (Utilities|Select :Index _index :Option%200 (Variables|Default|GetSM_Wood_0) :Option%201 (Variables|Default|GetSM_Wood_1) :Option%202 (Variables|Default|GetSM_Wood_2) :Option%203 (Variables|Default|GetSM_Wood_3) :Option%204 (Variables|Default|GetSM_Wood_4) :Option%205 (Variables|Default|GetSM_Wood_5) :Option%206 (Variables|Default|GetSM_Wood_6) :Option%207 (Variables|Default|GetSM_Wood_7) :Option%208 (Variables|Default|GetSM_Wood_8) :Option%209 (Variables|Default|GetSM_Wood_9)))))

(fn SetMoneyCubeArray
  (for _index (range 0 9)
    (Utilities|Array|AddUnique (Variables|Default|GetMoneyCubeArray) (Utilities|Select :Index _index :Option%200 (Variables|Default|GetSM_Money_0) :Option%201 (Variables|Default|GetSM_Money_1) :Option%202 (Variables|Default|GetSM_Money_2) :Option%203 (Variables|Default|GetSM_Money_3) :Option%204 (Variables|Default|GetSM_Money_4) :Option%205 (Variables|Default|GetSM_Money_5) :Option%206 (Variables|Default|GetSM_Money_6) :Option%207 (Variables|Default|GetSM_Money_7) :Option%208 (Variables|Default|GetSM_Money_8) :Option%209 (Variables|Default|GetSM_Money_9)))))