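; BP_MoneyBuilding is the bank building in the game, a child Blueprint of a parent building class.
; On BeginPlay it runs the parent logic, sets its building type and labels its WBP_BuildingName widget "BANK".
; The overlap and tick events are disabled and the construction script only calls the parent, so this Blueprint adds no other behavior.
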(event EventBeginPlay
  (|CallParentFunction)
  (Variables|Default|SetBuildingType 3)
  (bind _aswbp_building_name (Utilities|Casting|CastToWBP_BuildingName (UserInterface|GetWidget (Variables|Default|GetWidgetBuildingName))))
  (Rendering|Components|TextRender|SetText (Variables|/Game/ExtremeMining/UMG/WBP_BuildingName.WBP_BuildingName_C|GetBuildingNameText _aswbp_building_name) "BANK"))

(event Collision|EventActorBeginOverlap
  (params (OtherActor :type Actor%20Object%20Reference))
  (|CallParentFunction OtherActor) ; This node is disabled and will not be called.\nDrag off pins to build functionality.
)

(event EventTick
  (params (DeltaSeconds :type Float%20%28single-precision%29))
  (|CallParentFunction DeltaSeconds) ; This node is disabled and will not be called.\nDrag off pins to build functionality.
)

(fn ConstructionScript
  (|CallParentFunction))