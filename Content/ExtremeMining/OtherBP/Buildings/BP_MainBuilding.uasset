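; Main building that populates the colony with AI citizens and labels itself "MAIN".
; On BeginPlay it spawns the player state's starting citizens in a row and starts a looping one-second timer.
; A spawn check runs or cancels a timer for new citizens, based on the first storage building's food and the population cap, incrementing the citizen count on each spawn.
; Tick shows that timer's progress on a widget bar.
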(event Custom|CanWeSpawn
  ;[1 1 1] Spawn
  (bind _outactors (Actor|GetAllActorsOfClass "/Game/ExtremeMining/OtherBP/Buildings/BP_BuildingStorage.BP_BuildingStorage_C"))
  (bind _asemplayer_state (Utilities|Casting|CastToEMPlayerState (Game|GetPlayerState 0)))
  (if (and (> (Variables|/Script/ExtremeMining.EMBuildingStorage|GetFood (Utilities|Array|Get(acopy) _outactors)) 50) (< (Variables|/Script/ExtremeMining.EMPlayerState|GetCurrentCitizenCount _asemplayer_state) (Variables|/Script/ExtremeMining.EMPlayerState|GetMaxCitizenCount _asemplayer_state)))
    (if (not (Utilities|Time|IsTimerActivebyHandle (Variables|Default|GetSpawnTimer)))
      (bind _returnvalue (Utilities|Time|SetTimerbyEvent (EventDispatchers|CreateEvent :!event Custom|SpawnCitizen) (Variables|Default|GetSpawnTime)))
      (Variables|Default|SetSpawnTimer _returnvalue))
    (else
      (Utilities|Time|ClearandInvalidateTimerbyHandle (Variables|Default|GetSpawnTimer)))))

(event Custom|SpawnCitizen
  ;[1 1 1] Spawn
  (AI|SpawnAIFromClass "/Game/ExtremeMining/OtherBP/Characters/BP_Citizen.BP_Citizen_C" "/Game/ExtremeMining/OtherBP/Characters/BehavoirTree/BT_CitizenBehavoir.BT_CitizenBehavoir" (.location (Transformation|GetWorldTransform (Variables|Default|GetCollisionBoxComponent))) "0, 0, 0" false 0)
  (bind _asemplayer_state (Utilities|Casting|CastToEMPlayerState (Game|GetPlayerState 0)))
  (Class|EMPlayerState|IncrementCurrentCitizenCount _asemplayer_state))

(event EventBeginPlay
  (|CallParentFunction)
  (Utilities|FlowControl|Sequence
    (:then_0
      (Variables|Default|SetBuildingType 0)
      (bind _aswbp_building_name (Utilities|Casting|CastToWBP_BuildingName (UserInterface|GetWidget (Variables|Default|GetWidgetBuildingName))))
      (Rendering|Components|TextRender|SetText (Variables|/Game/ExtremeMining/UMG/WBP_BuildingName.WBP_BuildingName_C|GetBuildingNameText _aswbp_building_name) "MAIN"))
    (:then_1
      (Utilities|Time|SetTimerbyEvent (EventDispatchers|CreateEvent :!event Custom|CanWeSpawn) 1.0 true))
    (:then_2
      (bind _asemplayer_state (Utilities|Casting|CastToEMPlayerState (Game|GetPlayerState 0)))
      (bind _returnvalue (Class|EMPlayerState|GetStartCitizenCount _asemplayer_state))
      (for _index (range 1 _returnvalue)
        (AI|SpawnAIFromClass "/Game/ExtremeMining/OtherBP/Characters/BP_Citizen.BP_Citizen_C" "/Game/ExtremeMining/OtherBP/Characters/BehavoirTree/BT_CitizenBehavoir.BT_CitizenBehavoir" (Math|Vector|MakeVector -5e+02 (Variables|Default|GetLocation%20Y) 2e+02) "0, 0, 0" false 0)
        (Variables|Default|SetLocation%20Y (+ (Variables|Default|GetLocation%20Y) 7e+01))
        (bind _asemplayer_state_2 (Utilities|Casting|CastToEMPlayerState (Game|GetPlayerState 0)))
        (Class|EMPlayerState|IncrementCurrentCitizenCount _asemplayer_state_2)))
    (:then_3
      (Utilities|Casting|CastToBP_EMPlayerState (Game|GetPlayerState 0)))))

(event Collision|EventActorBeginOverlap
  (params (OtherActor :type Actor%20Object%20Reference))
  (|CallParentFunction OtherActor) ; This node is disabled and will not be called.\nDrag off pins to build functionality.
)

(event EventTick
  (params (DeltaSeconds :type Float%20%28single-precision%29))
  (bind _spawntimer (Variables|Default|GetSpawnTimer))
  (if (not (Class|KismetSystemLibrary|IsTimerPausedHandle _spawntimer))
    (bind _aswbp_spawn_progress_bar (Utilities|Casting|CastToWBP_SpawnProgressBar (UserInterface|GetWidget (Variables|Default|GetWidgetProgressBar))))
    (Progress|SetPercent (Variables|/Game/ExtremeMining/UMG/WBP_SpawnProgressBar.WBP_SpawnProgressBar_C|GetProgressBar _aswbp_spawn_progress_bar) (/ (Class|KismetSystemLibrary|GetTimerElapsedTimeHandle _spawntimer) (Variables|Default|GetSpawnTime)))))

(fn ConstructionScript
  (|CallParentFunction))