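; Base citizen character that runs BT_CitizenBehavoir on its AI controller, with role hats, move-command effects and resource-collection feedback.
; Looping timers set up at BeginPlay drive procedural movement animation: a timeline bobs the body mesh while moving and not hungry, and the body rotates at full walk speed.
; Collection feedback shows a rate and icon chosen by character or resource type on a widget component, faded and moved vertically by timelines.
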(event Custom|CheckVelocity
  (bind _runtimer (Variables|Default|GetRunTimer))
  ;[0.9836 0.4491 1] Jump moving
  (if (and (not (Variables|Default|GetIsHungry)) (> (Math|Vector|VectorLength (Transformation|GetVelocity)) 0.0))
    (Utilities|Time|UnpauseTimerbyHandle _runtimer)
    (else
      (Utilities|Time|PauseTimerbyHandle _runtimer))))

(event Custom|CharRun
  (bind _bodymeshcomponent (Variables|Default|GetBodyMeshComponent))
  (bind _relativelocation (Variables|/Script/Engine.SceneComponent|GetRelativeLocation _bodymeshcomponent))
  ;[0.9836 0.4491 1] Jump moving
  (bind _newtrack_0 (Timeline|Timeline_0 PlayFromStart)
    (:Update
      (Transformation|SetRelativeLocation _bodymeshcomponent (Math|Vector|MakeVector (.x _relativelocation) (.y _relativelocation) (* _newtrack_0 (Variables|Default|GetDelta))) false false))))

(event Custom|IsCommand
  (bind _bodymeshcomponent (Variables|Default|GetBodyMeshComponent))
  ;[0.9836 0.4491 1] Jump moving
  (if (and (Utilities|Enum|Equal(Enum) (Class|AIController|GetMoveStatus (AI|GetAIController self)) "Moving") (== (Variables|/Script/Engine.CharacterMovementComponent|GetMaxWalkSpeed (Variables|Character|GetCharacterMovement)) 6e+02))
    (Transformation|SetRelativeRotation _bodymeshcomponent "20.000000, 0, 0" false false)
    (else
      (Transformation|SetRelativeRotation _bodymeshcomponent "0, 0, 0" false false))))

(event EventBeginPlay
  (bind _self self)
  (bind _returnvalue (AI|GetAIController _self))
  (Utilities|FlowControl|Sequence
    (:then_1
      ;[1 0.3451 0.9437] Visual animation
      (Utilities|Time|SetTimerbyEvent (EventDispatchers|CreateEvent :!event Custom|IsCommand) 0.3 true)
      (Utilities|Time|SetTimerbyEvent (EventDispatchers|CreateEvent :!event Custom|CheckVelocity) 0.3 true)
      (bind _returnvalue_2 (Utilities|Time|SetTimerbyEvent (EventDispatchers|CreateEvent :!event Custom|CharRun) 0.5 true))
      (bind _output_get (Variables|Default|SetRunTimer _returnvalue_2))
      (Utilities|Time|PauseTimerbyHandle _output_get))
    (:then_3
      ;[1 1 1] RunBehavoirTree
      (Utilities|IsValid _returnvalue
        (:Is%20Valid
          (AI|RunBehaviorTree _returnvalue "/Game/ExtremeMining/OtherBP/Characters/BehavoirTree/BT_CitizenBehavoir.BT_CitizenBehavoir"))))))

(event EventSetCollectWidget
  (params (ResourceType :type Integer))
  (bind _widgetresourcecollecttext (Variables|Default|GetWidgetResourceCollectText))
  (bind _relativelocation (Variables|/Script/Engine.SceneComponent|GetRelativeLocation _widgetresourcecollecttext))
  ;[1 1 1] Collect resource
  (bind _aswbp_caracter_collect_resource (Utilities|Casting|CastToWBP_CaracterCollectResource (UserInterface|GetWidget (Variables|Default|GetWidgetResourceCollectText))))
  (Rendering|Components|TextRender|SetText (Variables|/Game/ExtremeMining/UMG/WBP_CaracterCollectResource.WBP_CaracterCollectResource_C|GetResourceCountTextBlock _aswbp_caracter_collect_resource) (Utilities|Text|ToText(Integer) (Utilities|Select :Index (Variables|Default|GetCharacterType) :Option%200 (Variables|Default|GetCollectionRateNotWorker) :Option%201 (Variables|Default|GetCollectionRateWorkerFood) :Option%202 (Variables|Default|GetCollectionRateWorkerWood) :Option%203 (Variables|Default|GetCollectionRateWorkerMoney))))
  (if (== (Variables|Default|GetCharacterType) 0)
    (Appearance|SetBrushfromTexture (Variables|/Game/ExtremeMining/UMG/WBP_CaracterCollectResource.WBP_CaracterCollectResource_C|GetImage _aswbp_caracter_collect_resource) (Utilities|Select :Index ResourceType :Option%200 0 :Option%201 "/Game/ExtremeMining/Texture/UMG/apple.apple" :Option%202 "/Game/ExtremeMining/Texture/UMG/wood.wood" :Option%203 "/Game/ExtremeMining/Texture/UMG/dollar.dollar") false)
    (else
      (Appearance|SetBrushfromTexture (Variables|/Game/ExtremeMining/UMG/WBP_CaracterCollectResource.WBP_CaracterCollectResource_C|GetImage _aswbp_caracter_collect_resource) (Utilities|Select :Index (Variables|Default|GetCharacterType) :Option%200 0 :Option%201 "/Game/ExtremeMining/Texture/UMG/apple.apple" :Option%202 "/Game/ExtremeMining/Texture/UMG/wood.wood" :Option%203 "/Game/ExtremeMining/Texture/UMG/dollar.dollar") false)))
  (Utilities|FlowControl|Sequence
    (:then_0
      (bind _newtrack_0 (Timeline|Timeline_1 PlayFromStart)
        (:Update
          (bind _aswbp_caracter_collect_resource_2 (Utilities|Casting|CastToWBP_CaracterCollectResource (UserInterface|GetWidget (Variables|Default|GetWidgetResourceCollectText))))
          (Widget|SetRenderOpacity (Variables|/Game/ExtremeMining/UMG/WBP_CaracterCollectResource.WBP_CaracterCollectResource_C|GetBorder_1 _aswbp_caracter_collect_resource_2) _newtrack_0))))
    (:then_1
      (bind _newtrack_0_2 (Timeline|Timeline_2 PlayFromStart)
        (:Update
          (Transformation|SetRelativeLocation _widgetresourcecollecttext (Math|Vector|MakeVector (.x _relativelocation) (.y _relativelocation) _newtrack_0_2) false false))))))

(event EventSpawnMoveCommandFX
  (bind _returnvalue (Game|SpawnActorfromClass "/Game/ExtremeMining/OtherBP/FX/BP_NSCommand.BP_NSCommand_C" (Math|Transform|MakeTransform (+ (Transformation|GetWorldLocation (Variables|Default|GetBodyMeshComponent)) "0,0,150.000000")) "Undefined" 0 0))
  (Transformation|AttachComponentToComponent _returnvalue (Variables|Default|GetBodyMeshComponent) "None" "KeepWorld" "KeepWorld" "KeepWorld" true))

(event EventSetCharacterRole
  (params (Type :type Integer))
  ;[1 0.4737 0.8007] Set character role
  (Components|StaticMesh|SetStaticMesh (Variables|Default|GetHatMeshComponent) (Utilities|Select :Index Type :Option%200 "/Game/ExtremeMining/Mesh/Hats/SM_CapHat.SM_CapHat" :Option%201 "/Game/ExtremeMining/Mesh/Hats/SM_FoodHat.SM_FoodHat" :Option%202 "/Game/ExtremeMining/Mesh/Hats/WoodHat3.WoodHat3" :Option%203 "/Game/ExtremeMining/Mesh/Hats/SM_MoneyHat.SM_MoneyHat" :Option%204 "/Game/ExtremeMining/Mesh/Hats/SM_SeaHat.SM_SeaHat")))

(fn ConstructionScript)