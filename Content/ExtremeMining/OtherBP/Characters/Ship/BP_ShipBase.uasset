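; Base ship Blueprint that provides sail, landing and cargo display helpers.
; Sail visibility works by swapping a mesh material slot between canvas and invisible materials.
; A visibility line trace between scene markers, dropped at the far end, decides whether the land button shows and records the passenger spawn point.
; Resource type and count drive a cargo mesh and widget component with icon and text, both hidden when the type is zero.
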(event EventSetResourceonBoardVisibility
  (params (InResourceType :type Integer) (InResourceCount :type Integer))
  (bind _transportedresourcemesh (Variables|Default|GetTransportedResourceMesh))
  (bind _transportedresourcewidget (Variables|Default|GetTransportedResourceWidget))
  (bind _aswbp_transported_resource (Utilities|Casting|CastToWBP_TransportedResource (UserInterface|GetWidget (Variables|Default|GetTransportedResourceWidget))))
  (Utilities|IsValid _aswbp_transported_resource
    (:Is%20Valid
      (if (!= InResourceType 0)
        (Utilities|FlowControl|Sequence
          (:then_0
            (Appearance|SetBrushfromTexture (Variables|/Game/ExtremeMining/UMG/WBP_TransportedResource.WBP_TransportedResource_C|GetResourceImage _aswbp_transported_resource) (Utilities|Select :Index InResourceType :Option%200 0 :Option%201 "/Game/ExtremeMining/Texture/UMG/Resources/apple.apple" :Option%202 "/Game/ExtremeMining/Texture/UMG/Resources/wood.wood" :Option%203 "/Game/ExtremeMining/Texture/UMG/Resources/dollar.dollar") false)
            (Rendering|Components|TextRender|SetText (Variables|/Game/ExtremeMining/UMG/WBP_TransportedResource.WBP_TransportedResource_C|GetResourceCountTextBlock _aswbp_transported_resource) (Utilities|Text|ToText(Integer) InResourceCount)))
          (:then_1
            (Rendering|SetVisibility _transportedresourcemesh true false)
            (Rendering|SetVisibility _transportedresourcewidget true false)))
        (else
          (Rendering|SetVisibility _transportedresourcemesh false false)
          (Rendering|SetVisibility _transportedresourcewidget false false))))))

(event EventSetLandButtonVisibitity
  (bind _returnvalue (Collision|LineTraceByChannel (Transformation|GetWorldLocation (Variables|Default|GetStartScene)) (+ (Transformation|GetWorldLocation (Variables|Default|GetEndScene)) "0,0,-500.000000") "TraceTypeQuery1" false 0 "None"))
  (Variables|Default|SetIsButtonVisible _returnvalue)
  (bind _output_get (Variables|Default|SetSpawnPassengersLocation (Transformation|GetWorldLocation (Variables|Default|GetStartScene)))))

(event EventSetSailVisual
  (params (IsVisible :type Boolean))
  (bind _bodymeshcomponent (Variables|Default|GetBodyMeshComponent))
  (if IsVisible
    (Rendering|Material|SetMaterial _bodymeshcomponent 1 "/Game/ExtremeMining/Materials/Other/MI_Canvas.MI_Canvas")
    (else
      (Rendering|Material|SetMaterial _bodymeshcomponent 1 "/Game/ExtremeMining/Materials/Other/MI_Invisible.MI_Invisible"))))

(fn ConstructionScript)