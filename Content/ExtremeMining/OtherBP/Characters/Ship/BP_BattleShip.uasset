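; BP_BattleShip is a ship Blueprint that fires broadside cannon volleys from its left or right side.
; CannonsVolleyAttack spawns a BP_Projectile at each of the chosen side's five scene-component locations, each with an attached BP_NSCommand.
; It then applies an impulse to every projectile's mesh along the hull's right vector, negated for left volleys and scaled by ImpulseForce.
; The impulse vector is also printed for debugging.
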(event EventBeginPlay)

(event Collision|EventActorBeginOverlap
  (params (OtherActor :type Actor%20Object%20Reference)))

(event EventTick
  (params (DeltaSeconds :type Float%20%28single-precision%29)))

(event EventCannonsVolleyAttack
  (params (InIsRight :type Boolean))
  (bind _impulseforce (Variables|Default|GetImpulseForce))
  (bind _impulseforce_2 (Variables|Default|GetImpulseForce))
  (bind _bodymeshcomponent (Variables|Default|GetBodyMeshComponent))
  (bind _returnvalue (Math|Vector|GetRightVector _bodymeshcomponent))
  (bind _returnvalue_2 (* _impulseforce -1.0))
  (Utilities|FlowControl|Sequence
    (:then_0
      (Utilities|Array|Clear (Variables|Default|GetProjectileArray)))
    (:then_1
      (for _array_element (select InIsRight (Utilities|Array|MakeArray (Variables|Default|GetScene1R) (Variables|Default|GetScene2R) (Variables|Default|GetScene3R) (Variables|Default|GetScene4R) (Variables|Default|GetScene5R)) (Utilities|Array|MakeArray (Variables|Default|GetScene1L) (Variables|Default|GetScene2L) (Variables|Default|GetScene3L) (Variables|Default|GetScene4L) (Variables|Default|GetScene5L)))
        (bind _returnvalue_3 (Game|SpawnActorfromClass "/Game/ExtremeMining/OtherBP/Characters/Ship/BP_Projectile.BP_Projectile_C" (Math|Transform|MakeTransform (Transformation|GetWorldLocation _array_element) "0, 0, 0" "1.000000,1.000000,1.000000") "Undefined" 0 0))
        (Utilities|Array|AddUnique (Variables|Default|GetProjectileArray) _returnvalue_3)
        (bind _returnvalue_4 (Game|SpawnActorfromClass "/Game/ExtremeMining/OtherBP/FX/BP_NSCommand.BP_NSCommand_C" (Transformation|GetActorTransform _returnvalue_3) "Undefined" 0 0))
        (Transformation|AttachActorToActor _returnvalue_4 _returnvalue_3 "None" "KeepWorld" "KeepWorld" "KeepWorld" true)))
    (:then_2
      (if InIsRight
        (Variables|Default|SetImpulseDirection (* _returnvalue (Math|Vector|MakeVector _impulseforce_2 _impulseforce_2 _impulseforce_2)))
        (else
          (Variables|Default|SetImpulseDirection (* _returnvalue (Math|Vector|MakeVector _returnvalue_2 _returnvalue_2 _returnvalue_2)))))
      (Development|PrintString (Utilities|String|ToString(Vector) (Variables|Default|GetImpulseDirection))))
    (:then_3
      (for _array_element_2 (Variables|Default|GetProjectileArray)
        (Physics|AddImpulse (Variables|/Game/ExtremeMining/OtherBP/Characters/Ship/BP_Projectile.BP_Projectile_C|GetStaticMesh _array_element_2) (Variables|Default|GetImpulseDirection) "None" false)))))

(fn ConstructionScript
  (|CallParentFunction))