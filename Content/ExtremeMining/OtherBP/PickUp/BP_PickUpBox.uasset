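; BP_PickUpBox is a resource pickup box whose decals show which resource type it holds.
; The SetTypeVisual event takes a resource type and selects a food, wood or money decal material, leaving the first option unset.
; It applies that material to all six decal components at once.
; Begin play, overlap and tick events are disabled, so the graph holds only this visual logic.
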(event EventBeginPlay)

(event Collision|EventActorBeginOverlap
  (params (OtherActor :type Actor%20Object%20Reference)))

(event EventTick
  (params (DeltaSeconds :type Float%20%28single-precision%29))
  (|CallParentFunction DeltaSeconds) ; This node is disabled and will not be called.\nDrag off pins to build functionality.
)

(event EventSetTypeVisual
  (params (InResourceType :type Integer))
  (Rendering|Components|Decal|SetDecalMaterial (Variables|Default|GetDecal1) (Utilities|Select :Index InResourceType :Option%200 0 :Option%201 "/Game/ExtremeMining/Materials/ResourceMaterial/MI_FoodDecal.MI_FoodDecal" :Option%202 "/Game/ExtremeMining/Materials/ResourceMaterial/MI_WoodDecal.MI_WoodDecal" :Option%203 "/Game/ExtremeMining/Materials/ResourceMaterial/MI_MoneyDecal.MI_MoneyDecal")))

(fn ConstructionScript
  (|CallParentFunction))